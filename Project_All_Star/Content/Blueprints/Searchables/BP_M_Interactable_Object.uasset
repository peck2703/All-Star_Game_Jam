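; Searchable interactable object for a horror game that the player can inspect to find a USB device.
; A collision component shows or hides its widget as the cached BP_Horror_Character player enters or leaves.
; Interact writes a found or nothing-found message to the player's main HUD, moving the HasUSB flag from object to player on success so the device is found only once.
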(event OnComponentBeginOverlap(Collision)
  (params (OverlappedComponent :type Primitive%20Component%20Object%20Reference) (OtherActor :type Actor%20Object%20Reference) (OtherComp :type Primitive%20Component%20Object%20Reference) (OtherBodyIndex :type Integer) (bFromSweep :type Boolean) (SweepResult :type Hit%20Result%20Structure%20%28by%20ref%29))
  (if (== OtherActor (Variables|Default|GetPlayer_Ref))
    (Rendering|SetVisibility (Variables|Default|GetWidget) true false)))

(event OnComponentEndOverlap(Collision)
  (params (OverlappedComponent :type Primitive%20Component%20Object%20Reference) (OtherActor :type Actor%20Object%20Reference) (OtherComp :type Primitive%20Component%20Object%20Reference) (OtherBodyIndex :type Integer))
  (if (== OtherActor (Variables|Default|GetPlayer_Ref))
    (Rendering|SetVisibility (Variables|Default|GetWidget) false false)))

(event EventBeginPlay
  (bind _asbp_horror_character (Utilities|Casting|CastToBP_Horror_Character (Game|GetPlayerCharacter 0)))
  (Variables|Default|SetPlayer_Ref _asbp_horror_character))

(event EventInteract
  (bind _player_ref (Variables|Default|GetPlayer_Ref))
  (bind _main_hud_ref (Variables|/Game/Blueprints/Characters/BP_Horror_Character.BP_Horror_Character_C|GetMain_HUD_Ref _player_ref))
  (if (Variables|Default|GetHas_USB?)
    (Variables|/Game/Blueprints/HUD/UI_Main_HUD.UI_Main_HUD_C|SetText_To_Display _main_hud_ref "USB Device Found!")
    (Variables|Default|SetHas_USB? false)
    (Variables|/Game/Blueprints/Characters/BP_Horror_Character.BP_Horror_Character_C|SetHasUSB (Variables|Default|GetPlayer_Ref) true)
    (else
      (Variables|/Game/Blueprints/HUD/UI_Main_HUD.UI_Main_HUD_C|SetText_To_Display _main_hud_ref "Nothing interesting was found."))))

(fn ConstructionScript)