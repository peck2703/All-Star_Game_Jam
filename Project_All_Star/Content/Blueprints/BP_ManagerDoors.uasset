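; Double door Blueprint for a horror game that swings two leaves, DoorL and DoorR, when Interact is called.
; The Door_Alpha timeline lerps each leaf's yaw in opposite directions from a shared angle.
; Interact reverses the timeline if closed and unlocked, clearing IsDoorClosed when finished; otherwise, including when locked, it sets IsDoorClosed and plays forward.
; BeginPlay caches the horror player character, which the graph never uses afterward.
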(event EventBeginPlay
  (bind _asbp_horror_character (Utilities|Casting|CastToBP_Horror_Character (Game|GetPlayerCharacter 0)))
  (Variables|Default|SetPlayer_Ref _asbp_horror_character))

(event EventInteract
  (if (and (Variables|Default|GetIsDoorClosed) (not (Variables|Default|GetIsLocked)))
    (bind (_direction _alpha) (Timeline|Door_Alpha Reverse)
      (:Update
        (Transformation|SetRelativeRotation (Variables|Default|GetDoor_L) (Math|Rotator|MakeRotator 0.0 0.0 (Math|Float|Lerp -9e+01 -2e+02 _alpha)) false false)
        (Transformation|SetRelativeRotation (Variables|Default|GetDoor_R) (Math|Rotator|MakeRotator 0.0 0.0 (Math|Float|Lerp -9e+01 1e+01 _alpha)) false false))
      (:Finished
        (switch Utilities|FlowControl|Switch|SwitchonETimelineDirection _direction
          (:Backward
            (Variables|Default|SetIsDoorClosed false)))))
    (else
      (Variables|Default|SetIsDoorClosed true)
      (Timeline|Door_Alpha Play))))

(fn ConstructionScript)