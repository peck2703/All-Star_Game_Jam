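; BP_Character_M is a character Blueprint that shows dialogue through its ACDialogue component when interacted with.
; BeginPlay caches the BP_Horror_Character as PlayerRef, and Interact shows a random or next line, depending on RandomDialog.
; UpdateDialog shows the next page when MultPages is set, otherwise flags DialogDone.
; Sequential dialogue is a stub returning empty text, and the random index range includes the array length, one past the last element.
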(event Custom|UpdateDialog
  (bind _ac_dialogue (Variables|Default|GetAC_Dialogue))
  (if (Variables|/Game/Blueprints/Characters/AC_Dialogue.AC_Dialogue_C|GetMult_Pages _ac_dialogue)
    (bind _nexttexttodisplay (CallFunction|GetNextDialoguefromArray))
    (Default|ShowDialog _ac_dialogue _nexttexttodisplay)
    (else
      (Variables|Default|SetDialogDone? true))))

(event EventBeginPlay
  (bind _returnvalue (Actor|GetActorOfClass "/Game/Blueprints/Characters/BP_Horror_Character.BP_Horror_Character_C"))
  (Variables|Default|SetPlayer_Ref _returnvalue))

(event EventInteract
  (bind _ac_dialogue (Variables|Default|GetAC_Dialogue))
  (Variables|Default|SetDialogDone? false)
  (Default|ShowDialog _ac_dialogue (CallFunction|GetDialogTextfromArray _ac_dialogue)))

(fn ConstructionScript)

(fn RandomArraySelection
  (params (TargetArray :type Array%20of%20Texts))
  (return (Math|Random|RandomIntegerinRange 0 (Utilities|Array|Length TargetArray))))

(fn GetDialogTextfromArray
  (params (Component_Ref :type AC%20Dialogue%20Object%20Reference))
  (bind _dialogue_options (Variables|/Game/Blueprints/Characters/AC_Dialogue.AC_Dialogue_C|GetDialogue_Options Component_Ref))
  ;[0 0 0 0.5] Get a random dialog option if bool check is selected, and return a random from an array. If not random, select next dialog from array/dialog tree.
  (if (Variables|/Game/Blueprints/Characters/AC_Dialogue.AC_Dialogue_C|GetRandom_Dialog? Component_Ref)
    (return (Utilities|Array|Get(acopy) _dialogue_options (CallFunction|RandomArraySelection _dialogue_options)))
    (else
      (bind _nexttexttodisplay (CallFunction|GetNextDialoguefromArray))
      (return _nexttexttodisplay))))

(fn GetNextDialoguefromArray
  ;[0 0 0 0.5] If we have dialogue trees, we will have to select the next dialogue from an array, or struct
  (return ""))