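; BP_Camera_M is a surveillance camera trap that takes over the player's view inside its box and shows a VHS HUD.
; A timeline glides the crosshair between random screen points, deprojecting it into a line trace that respawns the player if hit while moving.
; Meanwhile, a looping timer with randomized delays sphere-traces for BPI_Change_Mats actors to toggle a "hellscape" material change.
; The construction script sizes the box and offsets the camera toward a corner.
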(event OnComponentBeginOverlap(Box)
  (params (OverlappedComponent :type Primitive%20Component%20Object%20Reference) (OtherActor :type Actor%20Object%20Reference) (OtherComp :type Primitive%20Component%20Object%20Reference) (OtherBodyIndex :type Integer) (bFromSweep :type Boolean) (SweepResult :type Hit%20Result%20Structure%20%28by%20ref%29))
  ;[0 0 0 0.5] Begin Overlap. If character overlaps, camera perspective changes to camera. Line Trace begins
  (if (== OtherActor (Game|GetPlayerCharacter 0))
    (CallFunction|BeginLineTrace)
    (Game|Player|SetViewTargetwithBlend (Game|GetPlayerController 0) self (Variables|Default|GetBlend_Time) "VTBlend_Linear" 0.0 false)
    ;;[0 0 0 0.5] Change HUD Visibilities
    (Default|ChangeHUDVisibility (Variables|References|GetPlayer_Ref))
    (CallFunction|FlipFlopHUDVisibility)
    (Variables|Default|SetActive true)
    (bind _returnvalue (Utilities|Time|SetTimerbyEvent (delegate Custom|StartHellscapeTimer) 0.1 true))
    (Variables|Default|SetHellscapeTimerHandle _returnvalue)
    (Variables|Default|SetHellscapeCount 0)))

(event OnComponentEndOverlap(Box)
  (params (OverlappedComponent :type Primitive%20Component%20Object%20Reference) (OtherActor :type Actor%20Object%20Reference) (OtherComp :type Primitive%20Component%20Object%20Reference) (OtherBodyIndex :type Integer))
  ;[0 0 0 0.5] End Overlap. If character leaves box area, view switches back over to character, and line trace ends.
  (if (== OtherActor (Game|GetPlayerCharacter 0))
    (CallFunction|BeginLineTrace)
    (Game|Player|SetViewTargetwithBlend (Game|GetPlayerController 0) (Variables|References|GetPlayer_Ref) (Variables|Default|GetBlend_Time) "VTBlend_Linear" 0.0 false)
    (Default|ChangeHUDVisibility (Variables|References|GetPlayer_Ref))
    (CallFunction|FlipFlopHUDVisibility)
    (Variables|Default|SetActive false)
    (Utilities|Time|ClearandInvalidateTimerbyHandle (Variables|Default|GetHellscapeTimerHandle))))

(event Custom|BeginLineTrace
  ;[0 0 0 0.5] Begins the line trace. As long as the camera is "active" and cursor moving, it will check.
  (if (not (and (Variables|Default|GetIsMoving?) (Variables|Default|GetActive)))
    (CallFunction|StartMovingCrossHair)))

(event Custom|StartMovingCrossHair
  ;[0 0 0 0.5] Starts moving the Crosshairs in UI Widget for Camera. Takes in a starting (x,y), chooses a random new (x,y) and then vinterps to set a new position.
  (Variables|Default|SetIsMoving? true)
  (bind (_starting_x _starting_y _desired_x _desired_y) (CallFunction|MoveCrossHair))
  (bind _alpha_track (Timeline|Transition_CrossHair PlayFromStart)
    (:Update
      (Class|CanvasPanelSlot|SetPosition (Variables|References|GetCrossHairSlot_Ref) (Math|Vector2D|MakeVector2D (.x (Math|Vector|Lerp(Vector) (Math|Vector|MakeVector _starting_x _starting_y 0.0) (Math|Vector|MakeVector _desired_x _desired_y 0.0) _alpha_track)) (.y (Math|Vector|Lerp(Vector) (Math|Vector|MakeVector _starting_x _starting_y 0.0) (Math|Vector|MakeVector _desired_x _desired_y 0.0) _alpha_track))))
      (CallFunction|TraceAlongPath))
    (:Finished
      ;[0 0 0 0.5] If stopped and camera still active, continue moving cross-hair
      (Utilities|FlowControl|Delay 0.2)
      (bind _output_get (Variables|Default|SetIsMoving? false))
      (if (and (not _output_get) (Variables|Default|GetActive))
        (CallFunction|BeginLineTrace)))))

(event Custom|TraceAlongPath
  ;[0 0 0 0.5] Processes inputs from Line Trace
  (if (Variables|Default|GetIsMoving?)
    (CallFunction|CalculateArrowTrajectory)))

(event Custom|StartHellscapeTimer
  ;[0.15 0.15 0.15 0.5] Hellscape timer. Every so often, turn on the hellscape
  (Utilities|FlowControl|Delay (CallFunction|DelayonOffHellscape))
  (CallFunction|FindWallsandCarpetMaterials)
  (Math|Integer|IncrementInt (Variables|Default|GetHellscapeCount)))

(event EventBeginPlay
  ;[0 0 0 0.5] Begin Play. Gather up references
  (bind _returnvalue (UserInterface|CreateWidget "/Game/Blueprints/HUD/UI_VHS_HUD.UI_VHS_HUD_C"))
  (bind _output_get (Variables|References|SetVHS_Ref _returnvalue))
  (Variables|/Script/UMG.Widget|SetVisibility _output_get "Collapsed")
  (UserInterface|Viewport|AddtoViewport _output_get 1)
  (bind _returnvalue_2 (UserInterface|CreateWidget "/Game/Blueprints/HUD/UI_VHS_Filter.UI_VHS_Filter_C"))
  (bind _output_get_2 (Variables|References|SetFilter_Ref _returnvalue_2))
  (Widget|SetVisibility _output_get_2 "Collapsed")
  (UserInterface|Viewport|AddtoViewport _output_get_2 0)
  (bind _asbp_horror_character (Utilities|Casting|CastToBP_Horror_Character (Game|GetPlayerCharacter 0)))
  (Variables|References|SetPlayer_Ref _asbp_horror_character)
  (Variables|References|SetCrossHairSlot_Ref (Class|WidgetLayoutLibrary|SlotasCanvasSlot (Variables|/Game/Blueprints/HUD/UI_VHS_HUD.UI_VHS_HUD_C|GetCross_Hair_Slot (Variables|References|GetVHS_Ref))))
  ;;[0 0 0 0.5] Controls the speed of the timeline (higher speed, faster tracker
  (Components|Timeline|SetPlayRate (Variables|Default|GetTransition_CrossHair) (Variables|Default|GetSpeedTracer)))

(fn ConstructionScript
  (bind (_x_offset _y_offset) (CallFunction|CalculateCameraOffset))
  (Components|Box|SetBoxExtent (Variables|Default|GetBox) (Math|Vector|MakeVector (Variables|Collision|GetBox_Width) (Variables|Collision|GetBox_Length) (Variables|Collision|GetBox_Height)) true)
  (Transformation|AddWorldOffset (Variables|Default|GetStaticMesh) (Math|Vector|MakeVector _x_offset _y_offset (Variables|Collision|GetCameraOffset_Z)) false false)
  (Transformation|SetRelativeRotation (Variables|Default|GetCamera) (Math|Rotator|MakeRotator 0.0 -3e+01 45.0) false false))

(fn FlipFlopHUDVisibility
  (bind _vhs_ref (Variables|References|GetVHS_Ref))
  (bind _filter_ref (Variables|References|GetFilter_Ref))
  ;[0 0 0 0.5] Essentially Flip-Flops the current visibility between collapsed/visible.
  (Variables|/Script/UMG.Widget|SetVisibility _vhs_ref (select (Utilities|Enum|Equal(Enum) (Variables|/Script/UMG.Widget|GetVisibility _vhs_ref) "Visible") "Collapsed" "Visible"))
  (Variables|/Script/UMG.Widget|SetVisibility _filter_ref (select (Utilities|Enum|Equal(Enum) (Variables|/Script/UMG.Widget|GetVisibility _filter_ref) "Visible") "Collapsed" "Visible"))
  (return))

(fn CameraMaxTrace
  (bind _box (Variables|Default|GetBox))
  (bind _boxextent (Variables|/Script/Engine.BoxComponent|GetBoxExtent _box))
  (return (Math|Float|Sqrt (+ (Math|Float|Square (.x _boxextent)) (Math|Float|Square (.y _boxextent)) (Math|Float|Square (.z _boxextent))))))

(fn CalculateCameraOffset
  (bind _box (Variables|Default|GetBox))
  (bind _staticmesh (Variables|Default|GetStaticMesh))
  (bind _distancefromcorner (Variables|Collision|GetDistanceFromCorner))
  (bind _boxextent (Variables|/Script/Engine.BoxComponent|GetBoxExtent _box))
  (bind _relativelocation (Variables|/Script/Engine.SceneComponent|GetRelativeLocation _staticmesh))
  ;[0 0 0 0.5] Force an offset based on the Box Extent size.
  (bind _output_get (Variables|Collision|SetCameraOffset_X (+ (- (.x _relativelocation) (.x _boxextent)) _distancefromcorner)))
  (bind _output_get_2 (Variables|Collision|SetCameraOffset_Y (+ (- (.y _relativelocation) (.y _boxextent)) _distancefromcorner)))
  (return _output_get _output_get_2))

(fn CalculateArrowTrajectory
  (bind _returnvalue (Game|GetPlayerController 0))
  (bind _vhs_ref (Variables|References|GetVHS_Ref))
  (bind _cross_hair (Variables|/Game/Blueprints/HUD/UI_VHS_HUD.UI_VHS_HUD_C|GetCross_Hair _vhs_ref))
  (bind _cross_hair_height (Variables|/Game/Blueprints/HUD/UI_VHS_HUD.UI_VHS_HUD_C|GetCross_Hair_Height _vhs_ref))
  (bind _cross_hair_width (Variables|/Game/Blueprints/HUD/UI_VHS_HUD.UI_VHS_HUD_C|GetCross_Hair_Width _vhs_ref))
  (bind _returnvalue_2 (Class|Widget|GetCachedGeometry _cross_hair))
  (bind _returnvalue_3 (/ _cross_hair_height 4.0))
  (bind _returnvalue_4 (/ _cross_hair_width 4.0))
  (bind _pixelposition (Class|SlateBlueprintLibrary|LocaltoViewport _returnvalue_2))
  (bind _returnvalue_5 (+ (.x _pixelposition) _returnvalue_4))
  (bind _returnvalue_6 (+ _returnvalue_3 (.y _pixelposition)))
  (bind (_worldlocation _worlddirection) (Class|PlayerController|DeprojectScreenPositiontoWorld _returnvalue _returnvalue_5 _returnvalue_6))
  ;[0 0 0 0.5] Line trace, searching for player. If hit, and hit actor is player, proceed.
  (bind _outhit (Collision|LineTraceByChannel _worldlocation (+ _worldlocation (* _worlddirection 1e+04)) "TraceTypeQuery2" false 0 "None"))
  (if (and (.bBlockingHit (Collision|BreakHitResult _outhit)) (== (.HitActor (Collision|BreakHitResult _outhit)) (Game|GetPlayerCharacter 0)))
    ;[0 0 0 0.5] If caught, respawn
    (bind _player_caught (CallFunction|CheckPlayerMovement))
    (if _player_caught
      (Default|Respawn (Variables|References|GetPlayer_Ref)))))

(fn MoveCrossHair
  (bind _crosshairslot_ref (Variables|References|GetCrossHairSlot_Ref))
  (bind _vhs_ref (Variables|References|GetVHS_Ref))
  (bind _returnvalue (Class|CanvasPanelSlot|GetPosition _crosshairslot_ref))
  (bind _viewport_x (Variables|/Game/Blueprints/HUD/UI_VHS_HUD.UI_VHS_HUD_C|GetViewport_X _vhs_ref))
  (bind _viewport_y (Variables|/Game/Blueprints/HUD/UI_VHS_HUD.UI_VHS_HUD_C|GetViewport_Y _vhs_ref))
  (bind _cross_hair_height (Variables|/Game/Blueprints/HUD/UI_VHS_HUD.UI_VHS_HUD_C|GetCross_Hair_Height _vhs_ref))
  (bind _cross_hair_width (Variables|/Game/Blueprints/HUD/UI_VHS_HUD.UI_VHS_HUD_C|GetCross_Hair_Width _vhs_ref))
  ;[0 0 0 0.5] Gather and store variables holding position values
  (bind _output_get (LocalVariables|SetLocal_Pos_X (.x _returnvalue)))
  (bind _output_get_2 (LocalVariables|SetLocal_Pos_Y (.y _returnvalue)))
  (bind _output_get_3 (LocalVariables|SetDesired_Pos_X (Math|Random|RandomFloatinRange (* (+ _cross_hair_width _viewport_x) -1.0) (- _viewport_x _cross_hair_width))))
  (bind _output_get_4 (LocalVariables|SetDesired_Pos_Y (Math|Random|RandomFloatinRange (* (+ _cross_hair_height _viewport_y) -1.0) (- _viewport_y _cross_hair_height))))
  (return _output_get _output_get_2 _output_get_3 _output_get_4))

(fn CheckPlayerMovement
  (if (> (Math|Vector|VectorLength (Transformation|GetVelocity (Variables|References|GetPlayer_Ref))) 1.0)
    (bind _output_get (LocalVariables|SetPlayerCaught true))
    (return _output_get)
    (else
      (bind _output_get_2 (LocalVariables|SetPlayerCaught false))
      (return _output_get_2))))

(fn FindWallsandCarpetMaterials
  (bind _returnvalue (Transformation|GetActorLocation))
  (bind _outhits (Collision|MultiSphereTraceByChannel _returnvalue _returnvalue (Variables|Default|GetRadius) "TraceTypeQuery1" false (Utilities|Array|MakeArray self) "None"))
  (for _array_element _outhits
    (if (.bBlockingHit (Collision|BreakHitResult _array_element))
      (if (Utilities|DoesObjectImplementInterface (.HitActor (Collision|BreakHitResult _array_element)) "/Game/Blueprints/BPI_Change_Mats.BPI_Change_Mats_C")
        (Class|BPIChangeMats|ChangeMat(Message) (.HitActor (Collision|BreakHitResult _array_element)))
        (Development|PrintString "And Change!")))))

(fn HellscapeTimer)

(fn DelayonOffHellscape
  (if (== (Math|Integer|%(Integer) (Variables|Default|GetHellscapeCount) 2) 1)
    (return (Math|Random|RandomFloatinRange 0.5 2.0))
    (else
      (return (Math|Random|RandomFloatinRange 3.0 7.0)))))