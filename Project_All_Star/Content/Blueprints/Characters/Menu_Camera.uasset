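; Menu camera actor that drives the main menu, blending the player's view between the main, options and credits screens.
; On BeginPlay it creates the main menu widget with a reference to itself, adds it to the viewport, and switches to UI-only input with a visible cursor.
; SetActiveCamera collapses the menu, cubic-blends the view target to the chosen camera, then shows the menu again once the blend time elapses.
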(event Custom|SetActiveCamera
  (params (NewActiveCamera :type Main_Camera_Location%20Enum :default "NewEnumerator0"))
  (bind _returnvalue (Game|GetPlayerController 0))
  (bind _blendtimer (Variables|Movement|GetBlendTimer))
  ;[0 0 0 0.5] Set chosen camera to active, and all others inactive.
  (Widget|SetVisibility (Variables|Default|GetMain_Menu_Ref) "Collapsed")
  (switch Utilities|FlowControl|Switch|SwitchonMain_Camera_Location NewActiveCamera
    (:NewEnumerator0
      (Game|Player|SetViewTargetwithBlend _returnvalue self _blendtimer "VTBlend_Cubic" 0.0 false)
      (Utilities|FlowControl|Delay _blendtimer))
    (:NewEnumerator1
      (Game|Player|SetViewTargetwithBlend _returnvalue (Variables|Movement|GetOptions_Camera) _blendtimer "VTBlend_Cubic" 0.0 false)
      (Utilities|FlowControl|Delay _blendtimer))
    (:NewEnumerator2
      (Game|Player|SetViewTargetwithBlend _returnvalue (Variables|Movement|GetCredits_Camera) _blendtimer "VTBlend_Cubic" 0.0 false)
      (Utilities|FlowControl|Delay _blendtimer)))
  (Widget|SetVisibility (Variables|Default|GetMain_Menu_Ref) "Visible"))

(event EventBeginPlay
  (Input|SetInputModeUIOnly (Game|GetPlayerController 0) 0 "DoNotLock" false)
  (bind _returnvalue (UserInterface|CreateWidget "/Game/Blueprints/HUD/UI_Main_Menu.UI_Main_Menu_C" 0 self))
  (bind _output_get (Variables|Default|SetMain_Menu_Ref _returnvalue))
  (Default|SetReference _output_get self)
  (UserInterface|Viewport|AddtoViewport _output_get 0)
  (Variables|/Script/Engine.PlayerController|SetbShowMouseCursor (Game|GetPlayerController 0) true))

(fn ConstructionScript)