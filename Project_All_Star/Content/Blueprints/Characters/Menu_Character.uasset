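; Menu character Blueprint meant to show the main menu and blend the view between Main Menu, Options and Credits cameras.
; Its unconnected logic creates the UI_Main_Menu widget with UI-only input and a mouse cursor, and hides the widget during each timed view-target blend.
; Both BeginPlay and SetActiveCamera are empty, so none of this logic runs as wired.
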(event Custom|SetActiveCamera
  (params (NewActiveCamera :type Main_Camera_Location%20Enum :default "NewEnumerator0"))
  ;[0 0 0 0.5] Set chosen camera to active, and all others inactive.
)

(event EventBeginPlay)

(fn ConstructionScript)