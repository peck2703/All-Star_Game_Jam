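; BP_Monitor_Eyes is an interactable monitor that shows an eye widget while a camera actor has it activated.
; SetActive stores the camera, shows the eyes and raises its speed by 0.5.
; Interact hides the eyes and lowers speed even when inactive, but decrements the camera's monitor count only if active.
; The construction script sizes the Box, whose player-overlap check does nothing.
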(event OnComponentBeginOverlap(Box)
  (params (OverlappedComponent :type Primitive%20Component%20Object%20Reference) (OtherActor :type Actor%20Object%20Reference) (OtherComp :type Primitive%20Component%20Object%20Reference) (OtherBodyIndex :type Integer) (bFromSweep :type Boolean) (SweepResult :type Hit%20Result%20Structure%20%28by%20ref%29))
  (if (== OtherActor (Variables|Default|GetPlayer_ref))
    _))

(event Custom|SetActive
  (params (CameraActor :type BP%20Camera%20M%20Object%20Reference))
  (Variables|Default|SetCamera_Object_Ref CameraActor)
  (Variables|Default|SetIsActive true)
  (Rendering|SetVisibility (Variables|Default|GetEyeWidget) true false)
  (Default|AdjustSpeed (Variables|Default|GetCamera_Object_Ref) 0.5)
  (Development|PrintString "Harder Daddy"))

(event EventBeginPlay
  (Variables|Default|SetIsActive false)
  (Variables|Default|SetPlayer_ref (Game|GetPlayerCharacter 0)))

(event EventInteract
  (Default|AdjustSpeed (Variables|Default|GetCamera_Object_Ref) -0.5)
  (Rendering|SetVisibility (Variables|Default|GetEyeWidget) false false)
  (if (Variables|Default|GetIsActive)
    (Variables|Default|SetIsActive false)
    (Default|RemoveMonitorCount (Variables|Default|GetCamera_Object_Ref))))

(fn ConstructionScript
  (Components|Box|SetBoxExtent (Variables|Default|GetBox) (Variables|Default|GetBoxExtendSize) true))