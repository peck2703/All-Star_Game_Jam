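; Server rack prop for a server room, procedurally assembled in its construction script with no active gameplay logic.
; NumberOfServerSlots sets how many slot and cover mesh instances stack downward from the top at fixed spacing.
; The remaining height below them determines how many larger power unit instances are added at a sideways offset, so the rack's layout adapts to the slot count.
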(event EventBeginPlay)

(event Collision|EventActorBeginOverlap
  (params (OtherActor :type Actor%20Object%20Reference)))

(event EventTick
  (params (DeltaSeconds :type Float%20%28single-precision%29)))

(fn ConstructionScript
  (bind _numberofserverslots (Variables|Default|GetNumberOfServerSlots))
  ;[0 0 0 0.5] First attach the server slots every 4.5 units from the top
  (for _index (range 0 _numberofserverslots)
    (Components|InstancedStaticMesh|AddInstance (Variables|Default|GetServerSlots) (Math|Transform|MakeTransform (- "0.000000,0.000000,205.000000" (* _index (Math|Vector|MakeVector 0.0 0.0 4.5))) "0, 0, 0" "1.000000,1.000000,1.000000") false)
    (Components|InstancedStaticMesh|AddInstance (Variables|Default|GetServerSlotsCovers) (Math|Transform|MakeTransform (- "0.000000,0.000000,205.000000" (* _index (Math|Vector|MakeVector 0.0 0.0 4.5))) "0, 0, 0" "1.000000,1.000000,1.000000") false))
  (bind _output_get (LocalVariables|SetSpaceUsedUp (* (+ _numberofserverslots 1) 4.5)))
  (bind _output_get_2 (LocalVariables|SetPowerUnits (/ (- 194.0 _output_get) 9)))
  (for _index_2 (range 0 _output_get_2)
    (Components|InstancedStaticMesh|AddInstance (Variables|Default|GetServerPower) (Math|Transform|MakeTransform (Utilities|Operators|Subtract "0.000000,51.000000,205.000000" (Math|Vector|MakeVector 0.0 0.0 _output_get) (Math|Vector|MakeVector 0.0 0.0 (* _index_2 9))) "0, 0, 0" "1.000000,1.000000,1.000000") false)))