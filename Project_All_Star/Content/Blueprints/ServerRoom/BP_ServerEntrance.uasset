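; BP_ServerEntrance is an interactable server room entrance that opens a linked door when the player has the USB.
; Its box overlap shows and hides a prompt widget for the player and caches the BP_Horror_Character reference.
; On Interact, if that character's HasUSB is set, it plays a beep, unlocks DoorReference and calls Interact on that door.
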(event OnComponentBeginOverlap(Box)
  (params (OverlappedComponent :type Primitive%20Component%20Object%20Reference) (OtherActor :type Actor%20Object%20Reference) (OtherComp :type Primitive%20Component%20Object%20Reference) (OtherBodyIndex :type Integer) (bFromSweep :type Boolean) (SweepResult :type Hit%20Result%20Structure%20%28by%20ref%29))
  (if (== OtherActor (Game|GetPlayerCharacter 0))
    (Utilities|IsValid (Variables|Default|GetPlayer_Ref)
      (:Is%20Valid
        (Rendering|SetVisibility (Variables|Default|GetWidget) true false))
      (:Is%20Not%20Valid
        (bind _asbp_horror_character (Utilities|Casting|CastToBP_Horror_Character (Game|GetPlayerCharacter 0)))
        (Variables|Default|SetPlayer_Ref _asbp_horror_character)
        (Rendering|SetVisibility (Variables|Default|GetWidget) true false)))))

(event OnComponentEndOverlap(Box)
  (params (OverlappedComponent :type Primitive%20Component%20Object%20Reference) (OtherActor :type Actor%20Object%20Reference) (OtherComp :type Primitive%20Component%20Object%20Reference) (OtherBodyIndex :type Integer))
  (if (== OtherActor (Game|GetPlayerCharacter 0))
    (Utilities|IsValid (Variables|Default|GetPlayer_Ref)
      (:Is%20Valid
        (Rendering|SetVisibility (Variables|Default|GetWidget) false false))
      (:Is%20Not%20Valid
        (bind _asbp_horror_character (Utilities|Casting|CastToBP_Horror_Character (Game|GetPlayerCharacter 0)))
        (Variables|Default|SetPlayer_Ref _asbp_horror_character)
        (Rendering|SetVisibility (Variables|Default|GetWidget) false false)))))

(event EventBeginPlay)

(event EventInteract
  (bind _door_reference (Variables|Default|GetDoor_Reference))
  (if (Variables|/Game/Blueprints/Characters/BP_Horror_Character.BP_Horror_Character_C|GetHasUSB (Variables|Default|GetPlayer_Ref))
    (Audio|PlaySoundatLocation (Variables|Default|GetBeep_Sound) (Transformation|GetActorLocation) "0, 0, 0" 1.0 1.0 0.0 0 0 0 0)
    (Variables|/Game/Blueprints/BP_ManagerDoors.BP_ManagerDoors_C|SetIsLocked _door_reference false)
    (Default|Interact _door_reference)))

(fn ConstructionScript)