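; Automatic double sliding door Blueprint for the server room that opens when the player approaches.
; Overlap begin and end on the Collision component, filtered to PlayerRef, play and reverse the Door timeline.
; The timeline's Alpha drives lerps that slide DoorL and DoorR apart along relative Y in opposite directions.
; The Interact event is left empty, so the doors respond only to overlap.
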(event OnComponentEndOverlap(Collision)
  (params (OverlappedComponent :type Primitive%20Component%20Object%20Reference) (OtherActor :type Actor%20Object%20Reference) (OtherComp :type Primitive%20Component%20Object%20Reference) (OtherBodyIndex :type Integer))
  ;[0 0 0 0.5] Doors Open Automatically
  (if (== OtherActor (Variables|Default|GetPlayer_Ref))
    (bind _alpha (Timeline|Door Reverse)
      (:Update
        (Transformation|SetRelativeLocation (Variables|Default|GetDoor_L) (Math|Vector|MakeVector 0.0 (Math|Float|Lerp 0.0 7e+01 _alpha) 0.0) false false)
        (Transformation|SetRelativeLocation (Variables|Default|GetDoor_R) (Math|Vector|MakeVector 0.0 (Math|Float|Lerp 0.0 -7e+01 _alpha) 0.0) false false)))))

(event OnComponentBeginOverlap(Collision)
  (params (OverlappedComponent :type Primitive%20Component%20Object%20Reference) (OtherActor :type Actor%20Object%20Reference) (OtherComp :type Primitive%20Component%20Object%20Reference) (OtherBodyIndex :type Integer) (bFromSweep :type Boolean) (SweepResult :type Hit%20Result%20Structure%20%28by%20ref%29))
  ;[0 0 0 0.5] Doors Open Automatically
  (if (== OtherActor (Variables|Default|GetPlayer_Ref))
    (bind _alpha (Timeline|Door Play)
      (:Update
        (Transformation|SetRelativeLocation (Variables|Default|GetDoor_L) (Math|Vector|MakeVector 0.0 (Math|Float|Lerp 0.0 7e+01 _alpha) 0.0) false false)
        (Transformation|SetRelativeLocation (Variables|Default|GetDoor_R) (Math|Vector|MakeVector 0.0 (Math|Float|Lerp 0.0 -7e+01 _alpha) 0.0) false false)))))

(event EventBeginPlay
  (|CallParentFunction) ; This node is disabled and will not be called.\nDrag off pins to build functionality.
)

(event EventInteract)

(fn ConstructionScript
  (|CallParentFunction))