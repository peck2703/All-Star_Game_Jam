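; Wall actor Blueprint that toggles its look between two materials and can show a random decal on its surface.
; ChangeMat swaps slot 0 between OldMaterial and NewMaterial, hiding the decal when restoring the old one.
; AddDecals reveals the decal with a material from GrabRandomDecalAsset, which picks from DecalArray using an inclusive range up to Length, so the index can overrun.
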(event EventChangeMat
  (bind _wall (Variables|Default|GetWall))
  (if (== (Variables|Default|GetOld_Material) (Rendering|Material|GetMaterial _wall 0))
    (Rendering|Material|SetMaterial _wall 0 (Variables|Default|GetNew_Material))
    (else
      (Rendering|Material|SetMaterial _wall 0 (Variables|Default|GetOld_Material))
      (Rendering|SetVisibility (Variables|Default|GetDecal) false false))))

(event EventAddDecals
  (bind _decal (Variables|Default|GetDecal))
  ;[0 0 0 0.5] Add Decals to walls
  (Rendering|Components|Decal|SetDecalMaterial _decal (CallFunction|GrabRandomDecalAsset))
  (Rendering|SetVisibility _decal true false))

(event EventBeginPlay)

(fn ConstructionScript)

(fn GrabRandomDecalAsset
  (return (Utilities|Array|Get(acopy) (Variables|Default|GetDecal_Array) (Math|Random|RandomIntegerinRange 0 (Utilities|Array|Length (Variables|Default|GetDecal_Array))))))