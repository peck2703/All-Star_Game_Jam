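; Horror game mode Blueprint that sets up the menu view and hands control to the main character when play starts.
; BeginPlay points the player camera at a Menu_Camera, finds or spawns the BP_Horror_Character, and caches all BP_Camera_M actors.
; ChangePlayer possesses the character, switches to game-only input, then calls StartPlay on the character and every cached camera.
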(event Custom|ChangePlayer
  (bind _returnvalue (Game|GetPlayerController 0))
  (bind _main_character_ref (Variables|Default|GetMain_Character_Ref))
  ;[0 0 0 0.5] Move to Main Character Actor
  (Pawn|Possess _returnvalue _main_character_ref)
  (Input|SetInputModeGameOnly _returnvalue false)
  (Default|StartPlay _main_character_ref)
  (CallFunction|ActivateCameraReferences))

(event EventBeginPlay
  (bind _main_character_start (Variables|Default|GetMain_Character_Start))
  ;[0 0 0 0.5] Get the Main Character Reference. Activate and possess the main menu character, if one exists
  (bind _outactors (Actor|GetAllActorsOfClass "/Game/Blueprints/Characters/Menu_Camera.Menu_Camera_C"))
  (Utilities|IsValid (Utilities|Array|Get(acopy) _outactors)
    (:Is%20Valid
      (Game|Player|SetViewTargetwithBlend (Game|GetPlayerController 0) (Utilities|Array|Get(acopy) _outactors) 0.0 "VTBlend_Linear" 0.0 false))
    (:Is%20Not%20Valid
      _))
  (bind _outactors_2 (Actor|GetAllActorsOfClass "/Game/Blueprints/Characters/BP_Horror_Character.BP_Horror_Character_C"))
  (Utilities|IsValid (Utilities|Array|Get(acopy) _outactors_2)
    (:Is%20Valid
      (Variables|Default|SetMain_Character_Ref (Utilities|Array|Get(acopy) _outactors_2)))
    (:Is%20Not%20Valid
      (bind _returnvalue (Game|SpawnActorfromClass "/Game/Blueprints/Characters/BP_Horror_Character.BP_Horror_Character_C" _main_character_start "Undefined" "MultiplyWithRoot" 0 _main_character_start 0))
      (Variables|Default|SetMain_Character_Ref _returnvalue)))
  (bind _outactors_3 (Actor|GetAllActorsOfClass "/Game/Blueprints/Characters/BP_Camera_M.BP_Camera_M_C"))
  (Variables|Default|SetCamera_Actors_Array _outactors_3))

(fn ConstructionScript)

(fn ActivateCameraReferences
  (for _array_element (Variables|Default|GetCamera_Actors_Array)
    (Default|StartPlay _array_element))
  (return))