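; Test Blueprint with a wall that switches between two materials.
; The ChangeMat event compares the Wall's slot 0 material with OldMaterial and applies NewMaterial on a match, otherwise OldMaterial, so repeated calls toggle it.
; BeginPlay and the construction script are empty, and nothing in the Blueprint calls ChangeMat.
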(event EventChangeMat
  (bind _wall (Variables|Default|GetWall))
  (if (== (Variables|Default|GetOld_Material) (Rendering|Material|GetMaterial _wall 0))
    (Rendering|Material|SetMaterial _wall 0 (Variables|Default|GetNew_Material))
    (else
      (Rendering|Material|SetMaterial _wall 0 (Variables|Default|GetOld_Material)))))

(event EventBeginPlay)

(fn ConstructionScript)